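; Playable Tails character for a 2D side-scrolling platformer, with movement along world X and a jump commented as a double jump.
; BeginPlay adds the platformer Enhanced Input mapping context and prints the spawn location; move and jump actions drive standard Character movement.
; Tick yaws the sprite to face the X velocity and picks the idle, run or rolling-jump flipbook from falling state and speed.
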(event `self.ReceiveTick`
  (params (DeltaSeconds :type "Float (single-precision)"))
  (bind _returnvalue_x (`KismetMathLibrary.BreakVector` (`self.GetVelocity`)))
  (`SceneComponent.K2_SetWorldRotation` (`self.Sprite`) (`KismetMathLibrary.MakeRotator` 0.0 0.0 (`KismetMathLibrary.SelectFloat` 0.0 180.0 (>= _returnvalue_x 0.0))) false false)
  (`PaperFlipbookComponent.SetFlipbook` (`self.Sprite`) (select `bool` (`NavMovementComponent.IsFalling` (`self.CharacterMovement`)) :`false` (select `bool` (> (`KismetMathLibrary.Abs` _returnvalue_x) 0.0) :`false` "/Game/Modulo27/characterSprite/FlipBooks/tails_idle.tails_idle" :`true` "/Game/Modulo27/characterSprite/FlipBooks/tails_run.tails_run" :!type "PaperFlipbook Object Reference") :`true` "/Game/Modulo27/characterSprite/FlipBooks/tails_jump_rolling.tails_jump_rolling")))

(event `self.ReceiveBeginPlay`
  ; Adicioando inputs do  Player
  (bind _asplayer_controller (cast `PlayerController` (`self.GetController`)))
  (message `EnhancedInputSubsystemInterface.AddMappingContext` (pcsubsystem `EnhancedInputLocalPlayerSubsystem` _asplayer_controller) "/Game/Modulo27/characterSprite/FlipBooks/IMC_2dPlataform.IMC_2dPlataform" 0 (struct))
  (`KismetSystemLibrary.PrintString` (`KismetStringLibrary.Conv_VectorToString` (`self.K2_GetActorLocation`)) true true (struct :`G` 0.66 :`B` 1.0 :`A` 1.0) 200.0))

(event `EnhancedInput|/Game/Modulo27/characterSprite/FlipBooks/IA_jump`
  (params (ActionValue :type Boolean) (ElapsedSeconds :type "Float (double-precision)") (TriggeredSeconds :type "Float (double-precision)") (InputAction :type "InputAction Object Reference" :default "/Game/Modulo27/characterSprite/FlipBooks/IA_jump.IA_jump"))
  ; Tem pulo duplo
  (:`Started`
    (`self.Jump`)
    (`PaperFlipbookComponent.SetFlipbook` (`self.Sprite`) "/Game/Modulo27/characterSprite/FlipBooks/tails_jump_rolling.tails_jump_rolling"))
  (:`Canceled`
    (`self.StopJumping`)))

(event `EnhancedInput|/Game/Modulo27/characterSprite/FlipBooks/IA_move`
  (params (ActionValue :type "Float (double-precision)") (ElapsedSeconds :type "Float (double-precision)") (TriggeredSeconds :type "Float (double-precision)") (InputAction :type "InputAction Object Reference" :default "/Game/Modulo27/characterSprite/FlipBooks/IA_move.IA_move"))
  (:`Triggered`
    (`self.AddMovementInput` (1.0 0.0 0.0) ActionValue)))

(fn `UserConstructionScript`)